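; Enemy melee attack Gameplay Ability that turns the avatar toward its combat target and plays a random tagged attack montage.
; The Event.Montage.MeleeAttack gameplay event triggers a radius search for live players around the socket location resolved from a montage tag.
; Each player found gets a debug sphere and the ability's effect applied, then the ability ends.
; It also ends on montage interruption or when no montages exist.
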(event `self.K2_ActivateAbility`
  (bind _returnvalue (`self.GetAvatarActorFromActorInfo`))
  (bind _output_get (set `self.AvatarActor` _returnvalue))
  (bind _returnvalue_2 (message `EnemyInterface.GetTargetActor` _output_get))
  (bind _ascombat_interface (cast `CombatInterface` _returnvalue)
    (:`then`
      (`CombatInterface.FaceTarget` _ascombat_interface (`Actor.K2_GetActorLocation` _returnvalue_2))
      (bind _returnvalue_3 (`CombatInterface.GetTaggedMontages` _ascombat_interface))
      (if (> (`KismetArrayLibrary.Array_Length` _returnvalue_3) 0)
        (bind (_montage _montagetag) (break `TaggedMontage` (`KismetArrayLibrary.Array_Random` _returnvalue_3)))
        (set `self.Montage Tag` _montagetag)
        (`AbilityTask_PlayMontageAndWait.CreatePlayMontageAndWaitProxy` "None" _montage 1.0 "None" false :!label _label
          (:`then`
            (`AbilityTask_WaitGameplayEvent.WaitGameplayEvent` (struct :`TagName` "Event.Montage.MeleeAttack") null
              (:`EventReceived`
                (bind _returnvalue_4 (message `CombatInterface.GetSocketLocation` (`self.AvatarActor`) (`self.Montage Tag`)))
                (bind _outactors (`AuraAbilitySystermLibrary.GetLivePlayerWithinRadius` (`|MakeArray` (`self.AvatarActor`)) _returnvalue_4 (`self.Radius`) (`self.AvatarActor`)))
                (for _array_element _outactors
                  (`KismetSystemLibrary.DrawDebugSphere` (`Actor.K2_GetActorLocation` _array_element) 20.0 12 (struct :`R` 0.062411 :`G` 1.0 :`A` 1.0) 2.0)
                  (`self.ApplyEffectToTarget` (`AbilitySystemBlueprintLibrary.GetAbilitySystemComponent` _array_element)))
                (`self.K2_EndAbility`))))
          (:`OnInterrupted`
            (`self.K2_EndAbility`)))
        (else
          (`self.K2_EndAbility`))))
    (:`CastFailed`
      (goto _label))))