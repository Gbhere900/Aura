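; Gameplay ability for the enemy Shaman that summons random follower pawns.
; It faces the target, plays the summon montage and, on its attack event, shuffles the spawn locations.
; A delayed loop spawns an effect and a pawn at each, gives it a default controller and raises the caster's follower count, which its destruction lowers.
; The ability ends after the last spawn or on montage interruption.
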(event `self.K2_ActivateAbility`
  (bind _returnvalue (`self.GetAvatarActorFromActorInfo`))
  (bind _output (`|GetArrayItem` (`self.SpawnLocation`) (`self.TempCount`)))
  (bind _ascombat_interface (cast `CombatInterface` (`self.GetAvatarActorFromActorInfo`)))
  (set `self.As Combat Interface` _ascombat_interface)
  (set `self.TempCount` 0)
  (bind _returnvalue_2 (message `EnemyInterface.GetTargetActor` _returnvalue))
  (bind _ascombat_interface_2 (cast `CombatInterface` _returnvalue)
    (:`then`
      (`CombatInterface.FaceTarget` _ascombat_interface_2 (`Actor.K2_GetActorLocation` _returnvalue_2)))
    (:`CastFailed`
      _))
  (`AbilityTask_PlayMontageAndWait.CreatePlayMontageAndWaitProxy` "None" "/Game/Assets/Enemies/Shaman/Animations/AM_Shaman_Summon.AM_Shaman_Summon" 1.0 "None" false
    (:`then`
      (`AbilityTask_WaitGameplayEvent.WaitGameplayEvent` (struct :`TagName` "Montage.Attack.1") null
        (:`EventReceived`
          (bind _returnvalue_3 (`self.GetSpawnLocations`))
          (bind _output_get (set `self.SpawnLocation` _returnvalue_3))
          (`KismetArrayLibrary.Array_Shuffle` _output_get)
          (`NiagaraFunctionLibrary.SpawnSystemAtLocation` "/Game/Assets/Effects/Cursor/FX_Cursor.FX_Cursor" _output :!label _label)
          (bind _returnvalue_4 (`|SpawnActorFromClass` (`KismetArrayLibrary.Array_Random` (`self.SummonTarget`)) (`KismetMathLibrary.MakeTransform` (+ _output (0.0 0.0 50.0)) (`KismetMathLibrary.Conv_VectorToRotator` (- _output (`Actor.K2_GetActorLocation` (`self.GetAvatarActorFromActorInfo`))))) "Undefined" "MultiplyWithRoot" null null))
          (add `Actor.OnDestroyed` _returnvalue_4 (delegate `自定义事件`))
          (`CombatInterface.AddOrSubtractFollowerNum` (`self.As Combat Interface`) 1)
          (bind _aspawn (cast `Pawn` _returnvalue_4))
          (`Pawn.SpawnDefaultController` _aspawn)
          (bind _result (`/Engine/EditorBlueprintResources/StandardMacros.IncrementInt` (`self.TempCount`))
            (:`  `
              (if (< _result (`self.SpawnNum`))
                (`KismetSystemLibrary.Delay` 0.2)
                (goto _label)
                (else
                  (`self.K2_EndAbility`))))))))
    (:`OnInterrupted`
      (`self.K2_EndAbility`))))

(event `自定义事件`
  (params (DestroyedActor :type "Actor Object Reference"))
  (`CombatInterface.AddOrSubtractFollowerNum` (`self.As Combat Interface`) -1))