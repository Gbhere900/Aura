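; Enemy slingshot ranged attack ability that fires a projectile at the avatar's target actor.
; On activation it caches the target's location, turns to face it and plays a random tagged montage from the avatar.
; A montage-tag gameplay event triggers SpawnFireBLot from the weapon socket toward the cached position, with optional pitch override.
; The ability ends after firing, on montage interruption, or when no montages exist.
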(event `self.K2_ActivateAbility`
  (bind _returnvalue (message `EnemyInterface.GetTargetActor` (`self.GetAvatarActorFromActorInfo`)))
  (bind _returnvalue_2 (`Actor.K2_GetActorLocation` _returnvalue))
  (set `self.TargetPosition` _returnvalue_2)
  (message `CombatInterface.FaceTarget` (`self.GetAvatarActorFromActorInfo`) _returnvalue_2)
  (bind _returnvalue_3 (message `CombatInterface.GetTaggedMontages` (`self.GetAvatarActorFromActorInfo`)))
  (if (> (`KismetArrayLibrary.Array_Length` _returnvalue_3) 0)
    (bind (_montage _sockettag _montagetag) (break `TaggedMontage` (`KismetArrayLibrary.Array_Random` _returnvalue_3)))
    (`AbilityTask_PlayMontageAndWait.CreatePlayMontageAndWaitProxy` "None" _montage 1.0 "None" false
      (:`then`
        (`AbilityTask_WaitGameplayEvent.WaitGameplayEvent` _montagetag null
          (:`EventReceived`
            (`self.SpawnFireBLot` (`self.TargetPosition`) (struct :`TagName` "Socket.Weapon") (`self.Override Pitch`) (`self.Pitch`))
            (`self.K2_EndAbility`))))
      (:`OnInterrupted`
        (`self.K2_EndAbility`)))
    (else
      (`self.K2_EndAbility`))))