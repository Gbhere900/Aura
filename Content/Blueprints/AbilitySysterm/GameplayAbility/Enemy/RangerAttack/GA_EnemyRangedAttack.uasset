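; Enemy ranged attack gameplay ability that fires a firebolt at the avatar's current target.
; On activation it draws a debug sphere, stores the target's position, faces it and plays a random montage from the avatar's tagged montages.
; A Event.Montage.RangedAttack gameplay event triggers the firebolt spawn toward the stored position, then ends the ability.
; The ability also ends if the montage is interrupted or none exists.
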(event `self.K2_ActivateAbility`
  (`KismetSystemLibrary.DrawDebugSphere` (`Actor.K2_GetActorLocation` (`self.GetAvatarActorFromActorInfo`)) 100.0 12 (struct :`R` 1.0 :`G` 0.441731 :`A` 1.0) 2.0)
  (bind _returnvalue (message `EnemyInterface.GetTargetActor` (`self.GetAvatarActorFromActorInfo`)))
  (bind _returnvalue_2 (`Actor.K2_GetActorLocation` _returnvalue))
  (set `self.TargetPosition` _returnvalue_2)
  (message `CombatInterface.FaceTarget` (`self.GetAvatarActorFromActorInfo`) _returnvalue_2)
  (bind _returnvalue_3 (message `CombatInterface.GetTaggedMontages` (`self.GetAvatarActorFromActorInfo`)))
  (if (> (`KismetArrayLibrary.Array_Length` _returnvalue_3) 0)
    (`AbilityTask_PlayMontageAndWait.CreatePlayMontageAndWaitProxy` "None" (`.Montage` (break `TaggedMontage` (`KismetArrayLibrary.Array_Random` _returnvalue_3))) 1.0 "None" false
      (:`then`
        (`AbilityTask_WaitGameplayEvent.WaitGameplayEvent` (struct :`TagName` "Event.Montage.RangedAttack") null
          (:`EventReceived`
            (`self.SpawnFireBLot` (`self.TargetPosition`))
            (`self.K2_EndAbility`))))
      (:`OnInterrupted`
        (`self.K2_EndAbility`)))
    (else
      (`self.K2_EndAbility`))))