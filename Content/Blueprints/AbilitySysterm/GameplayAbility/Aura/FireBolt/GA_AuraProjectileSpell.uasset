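; Gameplay ability that casts Aura's FireBolt projectile at the point under the mouse.
; On activation it gets target data under the mouse, turns the avatar to face the hit point and plays the cast montage.
; A montage gameplay event then spawns the bolt from the weapon socket toward that point.
; The ability ends after a short delay, which a comment credits with fixing clients failing to fire.
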(event `self.K2_ActivateAbility`
  ;[1 1 1] 为什么客户端点击不会产生火球
  (bind (_asynctaskproxy _datahandle) (`TargetDataUnderMouse.CreateTargetDataUnderMouse`)
    (:`ValidData`
      (bind _ascombat_interface (cast `CombatInterface` (`self.GetAvatarActorFromActorInfo`)))
      (bind (_bblockinghit _binitialoverlap _time _distance _location _impactpoint) (`GameplayStatics.BreakHitResult` (`AbilitySystemBlueprintLibrary.GetHitResultFromTargetData` _datahandle)))
      (`CombatInterface.FaceTarget` _ascombat_interface _impactpoint)
      (`AbilityTask_PlayMontageAndWait.CreatePlayMontageAndWaitProxy` "None" "/Game/Assets/Characters/Aura/Animations/Abilities/AM_Cast_FIreBlot.AM_Cast_FIreBlot" 1.0 "None" false
        (:`then`
          (`AbilityTask_WaitGameplayEvent.WaitGameplayEvent` (struct :`TagName` "Event.Montage.FireBolt") null
            (:`then`
              (`KismetSystemLibrary.PrintText` "Spell"))
            (:`EventReceived`
              (`self.SpawnFireBLot` _impactpoint (struct :`TagName` "Socket.Weapon"))
              ;[1 1 1] 为什么这里加个Delay就解决了客户端不能发射的问题
              (`KismetSystemLibrary.Delay` 0.2)
              (`self.K2_EndAbility`))))))))