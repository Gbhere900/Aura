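; Actor that fades its static mesh out and back in by animating a material parameter.
; Construction stores the original materials and builds dynamic instances from faded material variants.
; FadeOut swaps in those instances and plays a timeline driving FadeValue, restoring the originals if it finishes at full value; Fadein reverses it.
; BeginPlay sends a fade-out message, then a fade-in after a short delay.
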(event `self.ReceiveBeginPlay`
  (message `/Game/Assets/Interface/BPI_Fade.FadeOut` self)
  (`KismetSystemLibrary.Delay` 1.0)
  (message `/Game/Assets/Interface/BPI_Fade.FadeIn` self))

(event `/Game/Assets/Interface/BPI_Fade.FadeOut`
  (for (_array_element _array_index) (`self.DynamicMaterialInstance`)
    (`PrimitiveComponent.SetMaterial` (`self.StaticMesh`) _array_index _array_element)
    (bind (_direction `_新建轨道_0`) (`Timeline|FadeOutFadeIn` :!via `PlayFromStart` :!label _label)
      (:`Update`
        (for _array_element_2 (`self.DynamicMaterialInstance`)
          (`MaterialInstanceDynamic.SetScalarParameterValue` _array_element_2 "FadeValue" `_新建轨道_0`)))
      (:`Finished`
        (if (>= `_新建轨道_0` 1.0)
          (for (_array_element_3 _array_index_2) (`self.Materials`)
            (`PrimitiveComponent.SetMaterial` (`self.StaticMesh`) _array_index_2 _array_element_3)))))))

(event `/Game/Assets/Interface/BPI_Fade.FadeIn`
  (goto _label :!via `ReverseFromEnd`))

(fn `UserConstructionScript`
  (set `self.Materials` (`MeshComponent.GetMaterials` (`self.StaticMesh`)))
  (for _array_element (`self.FadedMaterialInstance`)
    (bind _returnvalue (`KismetMaterialLibrary.CreateDynamicMaterialInstance` _array_element))
    (`KismetArrayLibrary.Array_Add` (`self.DynamicMaterialInstance`) _returnvalue)))