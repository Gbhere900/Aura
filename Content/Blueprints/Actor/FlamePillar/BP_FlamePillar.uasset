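; BP_FlamePillar is a flame pillar actor whose point light varies in intensity during play.
; The construction script sets the light to OriginalIntensity.
; On BeginPlay it randomly starts one of two timelines, which then hand off to each other on finish in an endless alternating loop.
; Each timeline's track supplies a coefficient that multiplies OriginalIntensity every update.
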(event `self.ReceiveBeginPlay`
  (switch `int` (`KismetMathLibrary.RandomIntegerInRange` 0 1)
    (:`0`
      (`self.PlayTimeLine1`))
    (:`1`
      (`self.PlayTimeLine2`))))

(event `PlayTimeLine1`
  (bind (_direction `_新建轨道_0`) (`Timeline|时间轴` :!via `PlayFromStart`)
    (:`Update`
      (set `self.IntensityCoefficient` `_新建轨道_0`)
      (`LightComponent.SetIntensity` (`self.PointLight`) (* (`self.IntensityCoefficient`) (`self.OriginalIntensity`))))
    (:`Finished`
      (`self.PlayTimeLine2`))))

(event `PlayTimeLine2`
  (bind (_direction `_新建轨道_0`) (`Timeline|时间轴_0` :!via `PlayFromStart`)
    (:`Update`
      (set `self.IntensityCoefficient` `_新建轨道_0`)
      (`LightComponent.SetIntensity` (`self.PointLight`) (* (`self.IntensityCoefficient`) (`self.OriginalIntensity`))))
    (:`Finished`
      (`self.PlayTimeLine1`))))

(fn `UserConstructionScript`
  (`LightComponent.SetIntensity` (`self.PointLight`) (`self.OriginalIntensity`)))